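; Tookabri character Blueprint that turns touch joystick and keyboard input into left/right movement state.
; Touch and possession events are forwarded to the UTC touch input and pawn possession manager components.
; The joystick X axis splits at a threshold into positive, negative and neutral, with DoOnce gates firing MoveRight or MoveLeft once until neutral resets them.
; The gates share the pressed-flag setters with the D and Q keys, which set only those flags.
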(event OnXAxisChanged(UTCJoystickComponent)
  (params (Value :type Float%20%28single-precision%29))
  (Utilities|UTCSplitAxis Value 0.5
    (:Positive
      (|DoOnceMultiInput :!label _label
        (:A%20Out
          (Class|TKCharacter|MoveRight)
          (Variables|Default|SetCH_RightPressed true :!label _label_2))
        (:Reset%20Out
          (Variables|Default|SetCH_RightPressed false))
        (:B%20Out
          (goto _label_2))))
    (:Negative
      (|DoOnceMultiInput :!label _label_3
        (:A%20Out
          (Class|TKCharacter|MoveLeft)
          (Variables|Default|SetCH_LeftPressed true :!label _label_4))
        (:Reset%20Out
          (Variables|Default|SetCH_LeftPressed false))
        (:B%20Out
          (goto _label_4))))
    (:Neutral
      (Utilities|FlowControl|Sequence
        (:then_0
          (goto _label Reset%20In))
        (:then_1
          (goto _label_3 Reset%20In))))))

(event EventBeginPlay)

(event Collision|EventActorBeginOverlap
  (params (OtherActor :type Actor%20Object%20Reference)))

(event EventPossessed
  (params (NewController :type Controller%20Object%20Reference))
  (Utilities|UTCPawnPossesionManager NewController (stale EventUnpossessed OldController)))

(event EventUnpossessed
  (params (OldController :type Controller%20Object%20Reference))
  (Utilities|UTCPawnPossesionManager (stale EventPossessed NewController) OldController) ; enters at Unpossesed
)

(event Input|KeyboardEvents|D
  (params (Key :type Key%20Structure))
  (:Pressed
    (Variables|Default|SetCH_RightPressed true))
  (:Released
    (Variables|Default|SetCH_RightPressed false)))

(event Input|KeyboardEvents|Q
  (params (Key :type Key%20Structure))
  (:Pressed
    (Variables|Default|SetCH_LeftPressed true))
  (:Released
    (Variables|Default|SetCH_LeftPressed false)))

(event Input|TouchEvents|InputTouch
  (params (Location :type Vector) (FingerIndex :type ETouchIndex%20Enum))
  (:Pressed
    (Utilities|UTCTouchInputManager Location FingerIndex :!label _label))
  (:Released
    (goto _label Released))
  (:Moved
    (goto _label Moved)))

(fn ConstructionScript)